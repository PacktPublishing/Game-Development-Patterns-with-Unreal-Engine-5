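; RTS player controller that lets the player select a unit and order it to move.
; Select traces for Pawns under the cursor and stores the hit actor only if it implements BPI_Units.
; Action sends that unit a stop message on press, then a move-location message with the cursor's Visibility hit on release.
; Helpers for moving the controller's own pawn and tracing touch input are defined but not called here.
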(event `InputAction|Select`
  (params (Key :type "Key Structure"))
  (bind (_hitresult _returnvalue) (`self.GetHitResultUnderCursorForObjects` (`|MakeArray` "ObjectTypeQuery3" :!type "EObjectTypeQuery Enum")))
  (bind (_bblockinghit _binitialoverlap _time _distance _location _impactpoint _normal _impactnormal _physmat _hitactor) (`GameplayStatics.BreakHitResult` _hitresult))
  ;[0.05098 0.05098 0.05098] Selection of Units on left click - Will only select actors which extend from pawn, checks to see if implements interface to determine if can be controlled.
  (:`Pressed`
    (if _returnvalue
      (if (`KismetSystemLibrary.DoesImplementInterface` _hitactor "/Game/RTS/Blueprints/BPI_Units.BPI_Units_C")
        (set `self.SelectedUnit` _hitactor)))))

(event `InputAction|Action`
  (params (Key :type "Key Structure"))
  (bind _selectedunit (`self.SelectedUnit`))
  ;[0.05098 0.05098 0.05098] Set Target Location for Movement. Stop event is called to stop movement immediately when the player right clicks.
  (:`Pressed`
    (message `/Game/RTS/Blueprints/BPI_Units.Stop` _selectedunit))
  (:`Released`
    (message `/Game/RTS/Blueprints/BPI_Units.SetMoveLocation` _selectedunit (`self.GetLocationUnderCursor`))))

(fn `FollowMouseOrFinger`
  (params (Location :type "Vector Structure"))
  (bind _returnvalue (`self.K2_GetPawn`))
  (`Pawn.AddMovementInput` _returnvalue (`KismetMathLibrary.GetDirectionUnitVector` (`self.K2_GetActorLocation` _returnvalue) Location) 1.0 false))

(fn `GetLocationUnderCursor`
  (returns (Location :type "Vector Structure"))
  (return (`.Location` (`GameplayStatics.BreakHitResult` (`self.GetHitResultUnderCursorByChannel` "TraceTypeQuery1")))))

(fn `GetLocationUnderFinger`
  (returns (Location :type "Vector Structure"))
  (return (`.Location` (`GameplayStatics.BreakHitResult` (`self.GetHitResultUnderFingerByChannel` "Touch1" "TraceTypeQuery1")))))

(fn `MoveToHitLocation`
  (params (Location :type "Vector Structure"))
  (`AIBlueprintHelperLibrary.SimpleMoveToLocation` self Location)
  (`NiagaraFunctionLibrary.SpawnSystemAtLocation` (`self.FXCursor`) Location))

(fn `UserConstructionScript`)