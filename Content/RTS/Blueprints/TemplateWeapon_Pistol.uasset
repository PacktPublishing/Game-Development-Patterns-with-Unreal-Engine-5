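; RTS pistol weapon Blueprint that extends a parent weapon with hitscan firing and sound feedback.
; Firing runs a Visibility line trace forward from FirePoint out to Range, ignoring the owner, and applies DamagePerHit to the actor it hits.
; The effects event plays a sound at the weapon's location, and reload calls the parent logic before playing its own sound.
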(event `self.PlayEffects`
  (`GameplayStatics.PlaySoundAtLocation` "/Engine/VREditor/Sounds/VR_teleport.VR_teleport" (`self.K2_GetActorLocation`) (struct) 1.0 1.0 0.0 null null null null))

(event `self.ProcessFiring`
  (bind __firepoint (`self._FirePoint`))
  (bind _returnvalue (`SceneComponent.K2_GetComponentLocation` __firepoint))
  (bind (_outhit _returnvalue_2) (`KismetSystemLibrary.LineTraceSingle` _returnvalue (+ _returnvalue (* (`SceneComponent.GetForwardVector` __firepoint) (`self._Range`))) "TraceTypeQuery1" false (`|MakeArray` (`self.GetOwner`))))
  (if _returnvalue_2
    (`GameplayStatics.ApplyDamage` (`.HitActor` (`GameplayStatics.BreakHitResult` _outhit)) (`self._DamagePerHit`))))

(event `self.Reload`
  (`parent.Reload`)
  (`GameplayStatics.PlaySoundAtLocation` "/Engine/VREditor/Sounds/UI/Gizmo_Handle_Clicked.Gizmo_Handle_Clicked" (`self.K2_GetActorLocation`) (struct) 1.0 1.0 0.0 null null null null))

(fn `UserConstructionScript`)