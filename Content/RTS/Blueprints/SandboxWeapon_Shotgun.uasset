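; Shotgun weapon for the RTS sandbox that fires a burst of pellets per shot.
; SandboxFire checks ammo, then runs one line trace per pellet along random directions in a cone around the fire point's forward vector.
; Each shot updates ammo and blocks firing, starting a timer to Handle_FireDelay based on rate of fire.
; A failed ammo check calls Reload with a click sound.
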(event `self.SandboxFire`
  (if (`self._CanFire`)
    (bind _returnvalue (`self.CheckAmmo`))
    (if _returnvalue
      (`self.PlaySound` "/Engine/VREditor/Sounds/VR_teleport.VR_teleport")
      (for _ (range 1 (+ (`self.NumberOfPellets`) 1))
        (`self.LinetraceOneShot` (`KismetMathLibrary.RandomUnitVectorInConeInDegrees` (`SceneComponent.GetForwardVector` (`self._FirePoint`)) (`self.HalfSpreadDegrees`))))
      (`self.UpdateAmmo`)
      (set `self._CanFire` false)
      (bind _returnvalue_2 (`KismetSystemLibrary.K2_SetTimer` null "Handle_FireDelay" (/ 1.0 (`self._RoF`))))
      (set `self._TimerFireDelay` _returnvalue_2)
      (else
        (`self.Reload`)
        (`self.PlaySound` "/Engine/VREditor/Sounds/UI/Gizmo_Handle_Clicked.Gizmo_Handle_Clicked")))))

(fn `UserConstructionScript`)