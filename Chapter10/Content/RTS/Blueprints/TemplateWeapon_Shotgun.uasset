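; Shotgun weapon template for the RTS game, overriding the parent weapon's firing, effects and reload events.
; Firing casts one Visibility line trace per pellet in a random cone from the fire point, ignoring the parent actor and applying per-hit damage to any actor struck.
; Traces leave timed debug lines, while effects and reload play sounds at the weapon, with reload also calling the parent logic.
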(event `self.PlayEffects`
  (`GameplayStatics.PlaySoundAtLocation` "/Engine/VREditor/Sounds/VR_teleport.VR_teleport" (`self.K2_GetActorLocation`) (struct) 1.0 1.0 0.0 null null null null))

(event `self.ProcessFiring`
  (bind __firepoint (`self._FirePoint`))
  (bind _returnvalue (`SceneComponent.K2_GetComponentLocation` __firepoint))
  (for _ (range 1 (+ (`self.NumberOfPellets`) 1))
    (bind _outhit (`KismetSystemLibrary.LineTraceSingle` _returnvalue (+ _returnvalue (* (`KismetMathLibrary.RandomUnitVectorInConeInDegrees` (`SceneComponent.GetForwardVector` __firepoint) (`self.HalfSpreadDegrees`)) (`self._Range`))) "TraceTypeQuery1" false (`|MakeArray` (`self.GetParentActor`)) "ForDuration" true (struct :`R` 0.016924 :`B` 1.0 :`A` 1.0) (struct :`R` 1.0 :`B` 0.745052 :`A` 1.0)))
    (bind (_bblockinghit _binitialoverlap _time _distance _location _impactpoint _normal _impactnormal _physmat _hitactor) (`GameplayStatics.BreakHitResult` _outhit))
    (`/Engine/EditorBlueprintResources/StandardMacros.IsValid` _hitactor
      (:`Is Valid`
        (`GameplayStatics.ApplyDamage` _hitactor (`self._DamagePerHit`))))))

(event `self.Reload`
  (`parent.Reload`)
  (`GameplayStatics.PlaySoundAtLocation` "/Engine/VREditor/Sounds/UI/Gizmo_Handle_Clicked.Gizmo_Handle_Clicked" (`self.K2_GetActorLocation`) (struct) 1.0 1.0 0.0 null null null null))

(fn `UserConstructionScript`)