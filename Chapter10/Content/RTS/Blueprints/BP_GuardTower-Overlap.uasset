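; BP_GuardTower-Overlap is a guard tower Blueprint that borrows a pooled cube when play begins and later returns it.
; After the parent BeginPlay and a short delay, it finds the level's ObjectPool actor and requests a "PooledCube".
; It teleports the cube high above the tower, waits briefly, then recycles it to the pool.
; The file contains no overlap logic despite its name.
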(event `self.ReceiveBeginPlay`
  (`parent.ReceiveBeginPlay`)
  (`KismetSystemLibrary.Delay` 0.2)
  (bind _returnvalue (`GameplayStatics.GetActorOfClass` "/Script/RTS_AI.ObjectPool"))
  (set `self.ObjectPool` _returnvalue)
  (bind _returnvalue_2 (`ObjectPool.GetPooledActor` (`self.ObjectPool`) "PooledCube"))
  (set `self.Cube` _returnvalue_2)
  (`self.K2_SetActorLocation` _returnvalue_2 (+ (`self.K2_GetActorLocation`) (0.0 0.0 1500.0)) false true)
  (`KismetSystemLibrary.Delay` 2.0)
  (`ObjectPool.RecycleActor` (`self.ObjectPool`) (`self.Cube`)))

(fn `UserConstructionScript`)