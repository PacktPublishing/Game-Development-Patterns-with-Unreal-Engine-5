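; BP_EnemyUnit is an enemy unit actor for an RTS, configured from a TypeData reference.
; On BeginPlay, if TypeData is valid, it sets the Health component's max health and applies two materials to the mesh.
; When the Health component signals death, the actor destroys itself.
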(event `self.ReceiveBeginPlay`
  (bind _typedata (`self.TypeData`))
  (bind _mesh (`self.Mesh`))
  (`/Engine/EditorBlueprintResources/StandardMacros.IsValid` _typedata
    (:`Is Valid`
      (`|ExecutionSequence`
        (:`then_0`
          (`HealthComponent.InitializeNewMaxHealth` (`self.Health`) (`EnemyType._Health` _typedata)))
        (:`then_1`
          (`PrimitiveComponent.SetMaterial` _mesh 0 (`EnemyType._Material1` _typedata)))
        (:`then_2`
          (`PrimitiveComponent.SetMaterial` _mesh 1 (`EnemyType._Material2` _typedata)))))))

(event `self.Health.onComponentDead`
  (params (causer :type "Controller Object Reference"))
  ;[1 0 0] Handle Unit Death
  (`self.K2_DestroyActor`))

(fn `UserConstructionScript`)