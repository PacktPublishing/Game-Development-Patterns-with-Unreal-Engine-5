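; Pistol weapon Blueprint for the RTS sandbox that fires a single line-trace shot from its fire point each time SandboxFire runs.
; When firing is allowed and ammo remains, it plays a sound, traces, updates ammo and starts a Handle_FireDelay timer based on rate of fire.
; An empty magazine triggers a reload with a different sound.
; Ammo, trace and reload logic are defined outside this graph.
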(event `self.SandboxFire`
  (if (`self._CanFire`)
    (bind _returnvalue (`self.CheckAmmo`))
    (if _returnvalue
      (`self.PlaySound` "/Engine/VREditor/Sounds/VR_teleport.VR_teleport")
      (`self.LinetraceOneShot` (`SceneComponent.GetForwardVector` (`self._FirePoint`)))
      (`self.UpdateAmmo`)
      (bind _returnvalue_2 (`KismetSystemLibrary.K2_SetTimer` null "Handle_FireDelay" (/ 1.0 (`self._RoF`))))
      (set `self._TimerFireDelay` _returnvalue_2)
      (else
        (`self.Reload`)
        (`self.PlaySound` "/Engine/VREditor/Sounds/UI/Gizmo_Handle_Clicked.Gizmo_Handle_Clicked")))))

(fn `UserConstructionScript`)