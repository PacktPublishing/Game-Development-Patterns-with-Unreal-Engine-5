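; BP_MovingBox_Bad is an example Blueprint that shuttles a static mesh box back and forth along the X axis.
; Every Tick offsets the relative location by a fixed step, with the Forward flag choosing direction, so speed depends on frame rate.
; The flag flips when the box matches EndPoint with zero tolerance or StartPoint with a small tolerance, with no clamping or overshoot handling.
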(event `self.ReceiveTick`
  (params (DeltaSeconds :type "Float (single-precision)"))
  (bind _staticmesh_box (`self.StaticMesh_Box`))
  (bind _staticmesh_box_2 (`self.StaticMesh_Box`))
  (if (`self.Forward`)
    (`SceneComponent.K2_SetRelativeLocation` _staticmesh_box_2 (+ (`SceneComponent.RelativeLocation` _staticmesh_box_2) (1.0 0.0 0.0)) false false)
    (if (== (`SceneComponent.RelativeLocation` (`self.StaticMesh_Box`)) (`self.EndPoint`) :`ErrorTolerance` 0.0)
      (set `self.Forward` false))
    (else
      (`SceneComponent.K2_SetRelativeLocation` _staticmesh_box (+ (`SceneComponent.RelativeLocation` _staticmesh_box) (-1.0 0.0 0.0)) false false)
      (if (== (`SceneComponent.RelativeLocation` (`self.StaticMesh_Box`)) (`self.StartPoint`) :`ErrorTolerance` 1.0)
        (set `self.Forward` true)))))

(fn `UserConstructionScript`)